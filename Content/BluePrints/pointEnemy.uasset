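; Enemy character that patrols back and forth along world X between two points either side of its spawn location.
; Tick re-issues AI MoveTo toward the current point unless stunned, and arrival flips the direction flag.
; Its Knockback event stuns it, subtracts the player's STR from Health, then destroys it or launches it along the player's forward vector.
; Capsule hits on the TopDownCharacter knock the player back and briefly pause the enemy.
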(event `self.ReceiveTick`
  (params (DeltaSeconds :type "Float (single-precision)"))
  (`KismetSystemLibrary.PrintString` (`KismetStringLibrary.Conv_VectorToString` (`self.originalLocation`)))
  (if (`self.EnemyStunned`)
    (`KismetSystemLibrary.PrintString` "enemy stunned false")
    (elif (`self.move direction`)
      (`self.move to target location `)
      (else
        (`self.move to target location 2`)))))

(event `move to target location`
  (`|AIMoveTo` self (stale `self.ReceiveBeginPlay` _output_get) null 0.5
    (:`OnSuccess`
      (`KismetSystemLibrary.Delay` 0.2)
      (`KismetSystemLibrary.PrintString` "reached target location")
      (set `self.move direction` false))))

(event `self.ReceiveBeginPlay`
  (bind _originallocation (`self.originalLocation`))
  (set `self.originalLocation` (`self.K2_GetActorLocation`))
  (`|ExecutionSequence`
    (:`then_0`
      (bind _output_get (set `self.target location` (+ _originallocation (100.0 0.0 0.0)))))
    (:`then_1`
      (bind _output_get_2 (set `self.target location2` (- _originallocation (100.0 0.0 0.0)))))))

(event `move to target location 2`
  (`|AIMoveTo` self (stale `self.ReceiveBeginPlay` _output_get_2) null 0.5
    (:`OnSuccess`
      (set `self.move direction` true))))

(event `stunned`
  (set `self.EnemyStunned` true)
  (`MovementComponent.StopMovementImmediately` (`self.CharacterMovement`))
  (`KismetSystemLibrary.Delay` 2.0)
  (set `self.EnemyStunned` false))

(event `cooldown`
  (set `self.EnemyStunned` true)
  (`MovementComponent.StopMovementImmediately` (`self.CharacterMovement`))
  (`KismetSystemLibrary.Delay` 1.0)
  (set `self.EnemyStunned` false))

(event `knockback`
  (bind _health (`self.health`))
  (`self.stunned`)
  (bind _astop_down_character (cast `/Game/BluePrints/TopDownCharacter` (`GameplayStatics.GetPlayerPawn` 0)))
  (set `self.health` (- _health (`/Game/BluePrints/TopDownCharacter.STR` _astop_down_character)))
  (if (<= _health 0)
    (`self.K2_DestroyActor`)
    (else
      (`self.LaunchCharacter` (* (`/Game/BluePrints/TopDownCharacter.forward vector` _astop_down_character) (1000.0 1000.0 1000.0))))))

(event `self.CapsuleComponent.OnComponentHit`
  (params (HitComponent :type "PrimitiveComponent Object Reference") (OtherActor :type "Actor Object Reference") (OtherComp :type "PrimitiveComponent Object Reference") (NormalImpulse :type "Vector Structure") (Hit :type "HitResult Structure (by ref)"))
  (bind _astop_down_character (cast `/Game/BluePrints/TopDownCharacter` OtherActor))
  (`/Game/BluePrints/TopDownCharacter.playerKnockback` _astop_down_character (`self.GetActorForwardVector`))
  (`self.cooldown`))

(fn `UserConstructionScript`)