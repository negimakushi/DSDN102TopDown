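; Base enemy Character for a top-down game that chases the player and trades knockback hits.
; Tick issues AIMoveTo toward the player pawn unless EnemyStunned is set by timed stun or cooldown events.
; The knockback event stuns it, subtracts the player's STR from Health, then destroys it or launches it along the player's forward vector.
; Capsule hits on the player trigger PlayerKnockback and a shorter self-cooldown.
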(event `self.ReceiveTick`
  (params (DeltaSeconds :type "Float (single-precision)"))
  (if (`self.EnemyStunned`)
    (`KismetSystemLibrary.PrintString` "enemy stunned false")
    (else
      (`|AIMoveTo` self (0.0 0.0 0.0) (`GameplayStatics.GetPlayerPawn` 0)))))

(event `stunned`
  (set `self.EnemyStunned` true)
  (`MovementComponent.StopMovementImmediately` (`self.CharacterMovement`))
  (`KismetSystemLibrary.Delay` 2.0)
  (set `self.EnemyStunned` false))

(event `cooldown`
  (set `self.EnemyStunned` true)
  (`MovementComponent.StopMovementImmediately` (`self.CharacterMovement`))
  (`KismetSystemLibrary.Delay` 1.0)
  (set `self.EnemyStunned` false))

(event `knockback`
  (bind _health (`self.health`))
  (`self.stunned`)
  (bind _astop_down_character (cast `/Game/BluePrints/TopDownCharacter` (`GameplayStatics.GetPlayerPawn` 0)))
  (set `self.health` (- _health (`/Game/BluePrints/TopDownCharacter.STR` _astop_down_character)))
  (if (<= _health 0)
    (`self.K2_DestroyActor`)
    (else
      (`self.LaunchCharacter` (* (`/Game/BluePrints/TopDownCharacter.forward vector` _astop_down_character) (1000.0 1000.0 1000.0))))))

(event `self.CapsuleComponent.OnComponentHit`
  (params (HitComponent :type "PrimitiveComponent Object Reference") (OtherActor :type "Actor Object Reference") (OtherComp :type "PrimitiveComponent Object Reference") (NormalImpulse :type "Vector Structure") (Hit :type "HitResult Structure (by ref)"))
  (bind _astop_down_character (cast `/Game/BluePrints/TopDownCharacter` OtherActor))
  (`/Game/BluePrints/TopDownCharacter.playerKnockback` _astop_down_character (`self.GetActorForwardVector`))
  (`self.cooldown`))

(fn `UserConstructionScript`)