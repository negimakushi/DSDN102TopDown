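; GameClear is an actor Blueprint that, despite its name, holds a health recovery action for the player's TopDownCharacter.
; Its Recoverly function casts the player pawn, adds a point of Health if below a fixed cap, prints the result, then destroys the actor.
; The event graph holds only disabled placeholder events, so nothing in this file calls Recoverly.
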(fn `recoverly`
  (bind _astop_down_character (cast `/Game/BluePrints/TopDownCharacter` (`GameplayStatics.GetPlayerPawn` 0)))
  (bind _health (`/Game/BluePrints/TopDownCharacter.health` _astop_down_character))
  (if (< _health 10)
    (bind _output_get (set `/Game/BluePrints/TopDownCharacter.health` (+ _health 1) _astop_down_character))
    (`KismetSystemLibrary.PrintString` "health +1")
    (else
      (`KismetSystemLibrary.PrintString` "health already max")))
  (`self.K2_DestroyActor`))

(fn `UserConstructionScript`)