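; Long pole item actor that can upgrade the player's TopDownCharacter and then remove itself.
; Longer increases the character's HitboxSize and GivePlayerSpeed raises its Speed by fixed steps, each destroying the item and printing a debug message.
; GetDestroyed removes the item without any effect.
; The event graph is empty, so these functions rely on external callers.
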(fn `Get destroyed`
  (`self.K2_DestroyActor`))

(fn `Give player speed`
  (bind _astop_down_character (cast `/Game/BluePrints/TopDownCharacter` (`GameplayStatics.GetPlayerPawn` 0)))
  (set `/Game/BluePrints/TopDownCharacter.Speed` (+ (`/Game/BluePrints/TopDownCharacter.Speed` _astop_down_character) 0.1) _astop_down_character)
  (`self.K2_DestroyActor`)
  (`KismetSystemLibrary.PrintString` "speed given"))

(fn `longer`
  (bind _astop_down_character (cast `/Game/BluePrints/TopDownCharacter` (`GameplayStatics.GetPlayerPawn` 0)))
  (set `/Game/BluePrints/TopDownCharacter.Hitbox size` (+ (`/Game/BluePrints/TopDownCharacter.Hitbox size` _astop_down_character) 5.0) _astop_down_character)
  (`self.K2_DestroyActor`)
  (`KismetSystemLibrary.PrintString` "get longer"))

(fn `UserConstructionScript`)